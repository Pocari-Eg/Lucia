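; BP_SkyBox_Space_R0 is a space skybox actor that displays a configurable starfield on its SkySphereSpace component.
; The Construction Script creates a dynamic instance of M_SkyBox_Space_R0_Inst, stores it as SkyMaterial and calls RefreshMaterial.
; RefreshMaterial pushes star color, tiling, speed and intensity variables into the material, with TilingU and TilingV cross-wired to the opposite axis parameters.
; The event graph holds only empty default events.
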(event EventBeginPlay)

(event Collision|EventActorBeginOverlap
  (params (OtherActor :type Actor%20Object%20Reference)))

(event EventTick
  (params (DeltaSeconds :type Float%20%28single-precision%29)))

(fn ConstructionScript
  (bind _returnvalue (Rendering|Material|CreateDynamicMaterialInstance (Variables|Default|GetSkySphere_Space) 0 "/Game/3DEnvironment/Level/SkyBox/M_SkyBox_Space_R0_Inst.M_SkyBox_Space_R0_Inst" "None" :!class /Script/Engine.PrimitiveComponent))
  (Variables|Default|SetSkyMaterial _returnvalue)
  (CallFunction|RefreshMaterial))

(fn RefreshMaterial
  (bind _skymaterial (Variables|Default|GetSkyMaterial))
  (Rendering|Material|SetVectorParameterValue _skymaterial "Star_Color" (Variables|Default|GetStar_Color) :!class /Script/Engine.MaterialInstanceDynamic)
  (Rendering|Material|SetScalarParameterValue _skymaterial "Tiling_U" (Variables|Default|GetTiling_V) :!class /Script/Engine.MaterialInstanceDynamic)
  (Rendering|Material|SetScalarParameterValue _skymaterial "Tiling_V" (Variables|Default|GetTiling_U) :!class /Script/Engine.MaterialInstanceDynamic)
  (Rendering|Material|SetScalarParameterValue _skymaterial "Star Speed" (Variables|Default|GetStar%20Speed) :!class /Script/Engine.MaterialInstanceDynamic)
  (Rendering|Material|SetScalarParameterValue _skymaterial "Star_int" (Variables|Default|GetStar_int) :!class /Script/Engine.MaterialInstanceDynamic))