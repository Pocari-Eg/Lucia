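; IreneSpirit is a short-lived ghost of Irene and her weapon that appears for attack combo steps.
; BeginPlay applies ghost-tail dynamic materials, with M_Emt on remaining slots, then waits a frame and picks one of three opacity timelines by attack count.
; The timeline toggles ghost visibility, keeps the player mesh visible and destroys the actor when finished.
; A fourth timeline drives a Tick lerp that nudges the capsule forward.
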(event EventTick
  (params (DeltaSeconds :type Float%20%28single-precision%29))
  (bind _returnvalue (Transformation|GetActorLocation))
  (Transformation|SetRelativeLocation (Variables|Default|GetCapsuleComponent) (Math|Vector|Lerp(Vector) _returnvalue (+ _returnvalue (* (Transformation|GetActorForwardVector) 3.0)) (stale EventBeginPlay _새_트랙_0)) false false))

(event EventBeginPlay
  (bind _returnvalue (Class|IreneSpirit|GetAttackCount))
  (bind _returnvalue_2 (Game|GetPlayerCharacter 0))
  (bind _mesh (Variables|Character|GetMesh))
  (bind _mesh_2 (Variables|Character|GetMesh))
  (bind _mesh_3 (Variables|/Script/Engine.Character|GetMesh _returnvalue_2))
  (Utilities|FlowControl|Sequence
    (:then_0
      (bind _returnvalue_3 (Rendering|Material|CreateDynamicMaterialInstance (Variables|Default|GetWeapon) 0 "/Game/Effect/MI_GhostTail1.MI_GhostTail1" "None" :!class /Script/Engine.PrimitiveComponent))
      (bind _returnvalue_4 (Rendering|Material|CreateDynamicMaterialInstance _mesh_2 0 "/Game/Effect/MI_GhostTail1.MI_GhostTail1" "None" :!class /Script/Engine.PrimitiveComponent))
      (bind _returnvalue_5 (Rendering|Material|CreateDynamicMaterialInstance _mesh_2 1 "/Game/Effect/MI_GhostTail1.MI_GhostTail1" "None" :!class /Script/Engine.PrimitiveComponent))
      (bind _returnvalue_6 (Rendering|Material|CreateDynamicMaterialInstance _mesh_2 2 "/Game/Effect/MI_GhostTail1.MI_GhostTail1" "None" :!class /Script/Engine.PrimitiveComponent))
      (Rendering|Material|CreateDynamicMaterialInstance _mesh_2 3 "/Game/Model/Irene/Material/M_Emt.M_Emt" "None" :!class /Script/Engine.PrimitiveComponent)
      (Rendering|Material|CreateDynamicMaterialInstance _mesh_2 4 "/Game/Model/Irene/Material/M_Emt.M_Emt" "None" :!class /Script/Engine.PrimitiveComponent)
      (Rendering|Material|CreateDynamicMaterialInstance _mesh_2 5 "/Game/Model/Irene/Material/M_Emt.M_Emt" "None" :!class /Script/Engine.PrimitiveComponent))
    (:then_1
      (Utilities|FlowControl|Delay (Utilities|Time|GetWorldDeltaSeconds))
      (Utilities|FlowControl|Sequence
        (:then_0
          (if (== _returnvalue 1)
            (bind _새_트랙_1 (Timeline|타임라인_0 Play)
              (:Update
                (Rendering|Material|SetScalarParameterValue _returnvalue_4 "Opacity" _새_트랙_1 :!class /Script/Engine.MaterialInstanceDynamic)
                (if (>= 0.0 _새_트랙_1)
                  (Rendering|SetVisibility _mesh_3 true true)
                  (Rendering|SetVisibility _mesh false true)
                  (else
                    (Rendering|SetVisibility _mesh_3 true true)
                    (Rendering|SetVisibility _mesh true true))))
              (:Finished
                (Class|IreneSpirit|SetDestroy)
                (Actor|DestroyActor)))))
        (:then_1
          (if (== _returnvalue 2)
            (bind _새_트랙_1_2 (Timeline|타임라인_1 Play)
              (:Update
                (Rendering|Material|SetScalarParameterValue _returnvalue_3 "Opacity" _새_트랙_1_2 :!class /Script/Engine.MaterialInstanceDynamic)
                (if (>= 0.0 _새_트랙_1_2)
                  (Rendering|SetVisibility _mesh_3 true true)
                  (Rendering|SetVisibility _mesh false true)
                  (else
                    (Rendering|SetVisibility _mesh_3 true true)
                    (Rendering|SetVisibility _mesh true true))))
              (:Finished
                (Class|IreneSpirit|SetDestroy)
                (Actor|DestroyActor)))))
        (:then_2
          (if (== _returnvalue 3)
            (bind _새_트랙_1_3 (Timeline|타임라인_2 Play)
              (:Update
                (Rendering|Material|SetScalarParameterValue _returnvalue_6 "Opacity" _새_트랙_1_3 :!class /Script/Engine.MaterialInstanceDynamic)
                (if (>= 0.0 _새_트랙_1_3)
                  (Rendering|SetVisibility _mesh_3 true true)
                  (Rendering|SetVisibility _mesh false true)
                  (else
                    (Rendering|SetVisibility _mesh_3 true true)
                    (Rendering|SetVisibility _mesh true true))))
              (:Finished
                (Class|IreneSpirit|SetDestroy)
                (Actor|DestroyActor)))))))
    (:then_2
      (bind _새_트랙_0 (Timeline|타임라인_3 PlayFromStart)))))

(fn ConstructionScript)