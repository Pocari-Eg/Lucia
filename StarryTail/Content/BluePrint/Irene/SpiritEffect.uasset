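; SpiritEffect is a projectile-like actor that flies forward and damages each Monster it passes through.
; Tick moves it a fixed step along its forward vector without sweeping or delta-time scaling, so its speed depends on frame rate.
; On overlap, it records new Monsters in an array so each is hit only once, applying fixed damage credited to the player pawn as causer and adding one stack count.
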(event EventBeginPlay)

(event Collision|EventActorBeginOverlap
  (params (OtherActor :type Actor%20Object%20Reference))
  (bind _asmonster (Utilities|Casting|CastToMonster OtherActor))
  (if (== (Utilities|Array|FindItem (Variables|Default|GetNewVar_0) _asmonster) -1)
    (Utilities|Array|Add (Variables|Default|GetNewVar_0) _asmonster)
    (Game|Damage|ApplyDamage _asmonster 8e+01 0 (Game|Player|GetPlayerPawn 0))
    (Class|Monster|AddStackCount _asmonster 1)))

(event EventTick
  (params (DeltaSeconds :type Float%20%28single-precision%29))
  (Transformation|SetActorLocation (+ (Transformation|GetActorLocation) (* (Transformation|GetActorForwardVector) 5e+01)) false false))

(fn ConstructionScript)