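; Player character Blueprint for Irene, handling presentation, UI hookup and debug shortcuts around events such as stances, perfect dodge, hits and healing.
; BeginPlay shows an intro scroll or tutorial widget, then forwards battle events to the in-game HUD.
; Timelines animate spring-arm zoom, camera rotation and material parameter collections for dodge and cloak effects, while timers end hit-stop done through CustomTimeDilation.
; Debug keys restart, heal or jump between levels and spawn points.
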(event Custom|FInGameBattle_Event_0
  (params (_FUNC :type Integer) (_CTIME :type Float%20%28single-precision%29))
  ;[0 0 0] 윤동욱 _ Ingame바인딩
  (bind _asbp_ingame (Utilities|Casting|CastToBP_Ingame (Variables|Default|GetmakeIngameWidget)))
  (switch int _FUNC
    (:1
      (Class|IngameWidgetD|STANCEGAUGEeCtime _asbp_ingame _CTIME))
    (:2
      (Class|IngameWidgetD|NORMALAttackCountMinus _asbp_ingame))
    (:3
      (Class|IngameWidgetD|NORMALAttackCountPlus _asbp_ingame))
    (:4
      (Class|IngameWidgetD|NORMALAttackCooltime _asbp_ingame _CTIME))
    (:5
      (Class|IngameWidgetD|ULTIMATEsetUltimate _asbp_ingame _CTIME))))

(event Custom|ScrollEndDsipatcher_Event
  (bind _returnvalue (UserInterface|CreateWidget "/Game/UI/BluePrint/Player/BP_TutorialWidget_D.BP_TutorialWidget_D_C"))
  (UserInterface|Viewport|AddtoViewport _returnvalue 0)
  (Class|IreneCharacter|SetIsPlay)
  ;[0 0 0] 윤동욱 _ Ingame바인딩
  (EventDispatchers|AssignFinGameBattle (delegate Custom|FInGameBattle_Event_0)))

(event EventBeginPlay
  (bind _stance_wing (Variables|IreneCharacter|GetStance_Wing))
  (bind _asstgame_instance (Utilities|Casting|CastToSTGameInstance (Game|GetGameInstance)))
  (bind _returnvalue (Class|STGameInstance|GetIsPlaying _asstgame_instance))
  (Utilities|FlowControl|Sequence
    (:then_0
      (if _returnvalue
        (bind _returnvalue_2 (UserInterface|CreateWidget "/Game/UI/BluePrint/Player/BP_TutorialWidget_D.BP_TutorialWidget_D_C"))
        (UserInterface|Viewport|AddtoViewport _returnvalue_2 0)
        (Class|IreneCharacter|SetIsPlay)
        ;[0 0 0] 윤동욱 _ Ingame바인딩
        (EventDispatchers|AssignFinGameBattle (delegate Custom|FInGameBattle_Event_0))
        (else
          (EventDispatchers|BindEventtoScrollEndDsipatcher (delegate Custom|ScrollEndDsipatcher_Event))
          (bind _returnvalue_3 (UserInterface|CreateWidget "/Game/UI/BluePrint/Player/BP_InfoScroll.BP_InfoScroll_C"))
          (UserInterface|Viewport|AddtoViewport _returnvalue_3 0))))
    (:then_1
      (Variables|Default|SetStance_Particle_Ring (Variables|IreneCharacter|GetStance_Ring))
      (Utilities|IsValid (Variables|Default|GetStance_Particle_Ring)
        (:Is%20Valid
          (Components|Activation|Deactivate (Variables|Default|GetStance_Particle_Ring)))))
    (:then_2
      (Variables|Default|SetDodge_Particle (Variables|Default|GetDodge_Test))
      (Utilities|IsValid (Variables|Default|GetDodge_Particle)
        (:Is%20Valid
          (Components|Activation|Deactivate (Variables|Default|GetDodge_Particle)))))
    (:then_3
      (Utilities|IsValid _stance_wing
        (:Is%20Valid
          (Components|Activation|Deactivate _stance_wing)
          (Components|Activation|Deactivate (Variables|Default|GetHP)))))))

(event EventWeaponVisible
  (params (Value :type Boolean))
  (bind _mesh (Variables|Character|GetMesh))
  ;[1 1 1] 코멘트
  (Effects|SpawnEmitterAttached "/Game/Effect/VFX_Irene/VFX_Sword/PS_Fire_Spawn.PS_Fire_Spawn" _mesh (Class|SkinnedMeshComponent|GetSocketBoneName _mesh "hand_rSwordSocket")))

(event EventLevelRestartEvent
  ;[1 1 1] 재시작
  (bind _asstgame_instance (Utilities|Casting|CastToSTGameInstance (Game|GetGameInstance)))
  (Class|STGameInstance|InitData _asstgame_instance)
  (Utilities|FlowControl|Delay 3.0)
  (Class|FMODBlueprintStatics|BusStopAllEvents "/Game/FMOD/Buses/Master.Master" "ALLOWFADEOUT")
  (bind _returnvalue (Game|GetCurrentLevelName true))
  (Game|OpenLevel(byName) (Utilities|String|StringToName _returnvalue)))

(event EventCameraOutEvent
  ;[1 1 1] Camera Zoom Out
  (if (Variables|Default|GetbIsRaidBattle)
    (Class|IreneCharacter|SetRaidBattleCamera)
    (else
      (Class|IreneCharacter|SetBattleCamera)))
  (bind _output_get (Variables|Default|SetOldDistance (Variables|/Script/Engine.SpringArmComponent|GetTargetArmLength (Variables|Default|GetSpringArmComp))))
  (Variables|Default|SetChangedDistance (- (.BattleCameraZPosition (Utilities|Struct|BreakPlayerCharacterDataStruct (Variables|Default|GetIreneData))) _output_get))
  (Variables|Default|SetbIsRaidBattle false)
  (bind _outtrack (Timeline|타임라인_0 Play)
    (:Update
      (Variables|/Script/Engine.SpringArmComponent|SetTargetArmLength (Variables|Default|GetSpringArmComp) (+ (Variables|Default|GetOldDistance) (* _outtrack (Variables|Default|GetChangedDistance)))))))

(event EventRaidBattleEvent
  ;[1 1 1] Camera Zoom Out
  (Variables|Default|SetbIsRaidBattle true))

(event EventCamerainEvent
  ;[1 1 1] Camera Zoom In
  (if (> (Variables|/Script/Engine.SpringArmComponent|GetTargetArmLength (Variables|Default|GetSpringArmComp)) (.MaxFollowCameraZPosition (Utilities|Struct|BreakPlayerCharacterDataStruct (Variables|Default|GetIreneData))))
    (bind _output_get (Variables|Default|SetOldDistance (Variables|/Script/Engine.SpringArmComponent|GetTargetArmLength (Variables|Default|GetSpringArmComp))))
    (Variables|Default|SetChangedDistance (- _output_get (Variables|Default|GetCameraz)))
    (bind _outtrack (Timeline|타임라인_1 PlayFromStart)
      (:Update
        (Variables|/Script/Engine.SpringArmComponent|SetTargetArmLength (Variables|Default|GetSpringArmComp) (- (Variables|Default|GetOldDistance) (* _outtrack (Variables|Default|GetChangedDistance))))))))

(event EventWaveEndEvent
  (Camera|PlayWorldCameraShake "/Game/BluePrint/Shake/Test_Shake3.Test_Shake3_C" "-18512.000000,-44415.000000,2236.000000" 0.0 5e+03)
  (bind _outactors (Actor|GetAllActorsOfClass "/Game/BluePrint/Object/BP_Dust_Bust_Lab_2.BP_Dust_Bust_Lab_2_C"))
  (Default|SpanwDustAEvent _outactors))

(event EventTick
  (params (DeltaSeconds :type Float%20%28single-precision%29))
  (Rendering|Material|SetScalarParameterValue "/Game/Model/Lucia/MFC_Player_Camera.MFC_Player_Camera" "Optys" (- (/ (Math|Vector|Distance(Vector) (Transformation|GetWorldLocation (Variables|Default|GetCapsuleComponent)) (Transformation|GetWorldLocation (Variables|Default|GetCameraComp))) 1e+01) 7.8) :!class /Script/Engine.KismetMaterialLibrary))

(event EventPerfectDodgeTimeEnd
  ;[1 1 1] 코멘트
)

(event EventHPRecoveringStart
  (bind _hp (Variables|Default|GetHP))
  (Effects|SpawnEmitterAttached "/Game/Effect/VFX_Irene/PS_Item_Hp_Bust.PS_Item_Hp_Bust" _hp "None")
  (Components|Activation|SetActive _hp true false))

(event EventPerfectDodgeStart
  ;[1 1 1] 코멘트
  (Utilities|FlowControl|Sequence
    (:then_0
      (Components|Activation|SetActive (Variables|Default|GetDodge_Particle) true false)
      (Rendering|Material|SetScalarParameterValue "/Game/Effect/MC_Ghost.MC_Ghost" "Opacity" 1.0 :!class /Script/Engine.KismetMaterialLibrary)
      (bind _새_트랙_0 (Timeline|타임라인_3 PlayFromStart)
        (:Update
          (Rendering|Material|SetScalarParameterValue "/Game/PostPocessFX/MF_Softdark.MF_Softdark" "Power" _새_트랙_0 :!class /Script/Engine.KismetMaterialLibrary))))))

(event EventHPRecoveringEnd
  (Development|PrintText "KILLHEAL")
  (Components|Activation|Deactivate (Variables|Default|GetHP)))

(event EventCreateTailEvent
  ;[1 1 1] 코멘트
  (bind _returnvalue (Game|SpawnActorfromClass "/Game/BluePrint/Irene/BP_Ghost.BP_Ghost_C" (Transformation|GetWorldTransform (Variables|Character|GetMesh)) "Undefined" 0 0))
  (Default|InitEvent _returnvalue (Variables|Character|GetMesh)))

(event EventPerfectDodgeAttackEnd
  ;[1 1 1] 코멘트
  (Utilities|FlowControl|Sequence
    (:then_0
      (bind _새_트랙_0 (Timeline|타임라인_3 Stop)
        (:Update
          (Rendering|Material|SetScalarParameterValue "/Game/PostPocessFX/MF_Softdark.MF_Softdark" "Power" _새_트랙_0 :!class /Script/Engine.KismetMaterialLibrary))))
    (:then_1
      (Rendering|Material|SetScalarParameterValue "/Game/PostPocessFX/MF_Softdark.MF_Softdark" "Power" 1.0 :!class /Script/Engine.KismetMaterialLibrary)
      (bind _새_트랙_0_2 (Timeline|타임라인_4 PlayFromStart)
        (:Update
          (Rendering|Material|SetScalarParameterValue "/Game/PostPocessFX/MF_Softdark.MF_Softdark" "Power" _새_트랙_0_2 :!class /Script/Engine.KismetMaterialLibrary))))
    (:then_2
      (bind _새_트랙_0_3 (Timeline|타임라인_5 PlayFromStart)
        (:Update
          (Rendering|Material|SetScalarParameterValue "/Game/Effect/MC_Ghost.MC_Ghost" "Opacity" _새_트랙_0_3 :!class /Script/Engine.KismetMaterialLibrary))))))

(event EventHitEffect
  ;[1 1 1] Hit Effet
  (Effects|SpawnEmitterAttached "/Game/Effect/VFX_Hit/PS_Player_Hit.PS_Player_Hit" (Variables|Character|GetMesh) "None" "0,0.000000,100.000000"))

(event EventHitStopEvent
  ;[1 1 1] Hit_Stop
  (if (not (Variables|Default|GetIsTimeStopping))
    (Utilities|FlowControl|Delay 0.05)
    (CallFunction|StartHitStop 0.1)))

(event EventRadialBlurEvent
  ;[1 1 1] RadialBlur
  (bind _returnvalue (Rendering|Material|GetScalarParameterValue "/Game/UI/RadialBlur/RadialBlurCollection.RadialBlurCollection" "Blur" :!class /Script/Engine.KismetMaterialLibrary))
  (if (== _returnvalue 0.0)
    (CallFunction|RadialBlurStart 0.3)))

(event EventInitComplete
  ;[1 1 1] UI
  (Utilities|FlowControl|Delay 0.01)
  (Default|CallPlayerInitDispatcher))

(event EventPlayFadeOutEvent
  ;[1 1 1] UI
  (bind _asbp_player_hud (Utilities|Casting|CastToBP_PlayerHud (Variables|/Script/Lucia.IreneUIManager|GetPlayerHud (Variables|Default|GetIreneUIManager))))
  (Default|FadeOutAnimationStart _asbp_player_hud))

(event EventNormalStance
  (bind _stance_particle_par (Variables|Default|GetStance_Particle_Par))
  (Utilities|IsValid _stance_particle_par
    (:Is%20Valid
      (Components|Activation|Deactivate _stance_particle_par)
      (Effects|SpawnEmitterAttached "/Game/Effect/VFX_Irene/Stance/Ps_Out_test.Ps_Out_test" (Variables|Character|GetMesh) "None" "0.000000, 0,1.000000")
      (bind _새_트랙_0 (Timeline|타임라인_7 PlayFromStart)
        (:Update
          (Rendering|Material|SetScalarParameterValue "/Game/Model/Lucia/MFC_Cloak_Power.MFC_Cloak_Power" "Opty" _새_트랙_0 :!class /Script/Engine.KismetMaterialLibrary))))))

(event EventSpiritStance
  (Utilities|FlowControl|Sequence
    (:then_0
      (bind _returnvalue (Effects|SpawnEmitterAttached "/Game/Effect/VFX_Irene/Stance/PS_TestPattern.PS_TestPattern" (Variables|Character|GetMesh) "None" "0, 0,1.000000"))
      (Variables|Default|SetStance_Particle_Par _returnvalue)
      (Utilities|FlowControl|Delay 0.5)
      (Components|Activation|SetActive (Variables|IreneCharacter|GetStance_Ring) true false))
    (:then_1
      (bind _새_트랙_0 (Timeline|타임라인_6 PlayFromStart)
        (:Update
          (Rendering|Material|SetScalarParameterValue "/Game/Model/Lucia/MFC_Cloak_Power.MFC_Cloak_Power" "Opty" _새_트랙_0 :!class /Script/Engine.KismetMaterialLibrary))))))

(event EventGameClearEvent
  ;[1 1 1] UI
  (Default|CallGameClearDispatcher))

(event Input|KeyboardEvents|F9
  (params (Key :type Key%20Structure :default "None"))
  (:Pressed
    (bind _asstgame_instance (Utilities|Casting|CastToSTGameInstance (Game|GetGameInstance)))
    (Class|STGameInstance|InitData _asstgame_instance)
    (Class|FMODBlueprintStatics|BusStopAllEvents "/Game/FMOD/Buses/Master.Master" "ALLOWFADEOUT")
    (bind _returnvalue (Game|GetCurrentLevelName true))
    (Game|OpenLevel(byName) (Utilities|String|StringToName _returnvalue))))

(event Input|KeyboardEvents|X
  (params (Key :type Key%20Structure :default "None"))
  ;[1 1 1] CameraRotaion
  (:Pressed
    (Variables|Default|SetTotalRotation 0.0)
    (bind _returnvalue (Class|IreneCharacter|BattleCameraRotation (Variables|Default|GetRotationAngel)))
    (bind _새_트랙_0 (Timeline|타임라인_2 PlayFromStart)
      (:Update
        (Pawn|Input|AddControllerYawInput (- (* _returnvalue _새_트랙_0) (Variables|Default|GetTotalRotation)))
        (Variables|Default|SetTotalRotation (* _returnvalue _새_트랙_0))))))

(event Input|KeyboardEvents|Ctrl3
  (params (Key :type Key%20Structure :default "None"))
  (:Pressed
    (Class|FMODBlueprintStatics|BusStopAllEvents "/Game/FMOD/Buses/Master.Master" "ALLOWFADEOUT")
    (bind _asstgame_instance (Utilities|Casting|CastToSTGameInstance (Game|GetGameInstance)))
    (Class|STGameInstance|InitData _asstgame_instance)
    (Game|OpenLevel(byName) "FairyBoss")))

(event Input|KeyboardEvents|F5
  (params (Key :type Key%20Structure :default "None"))
  (:Pressed
    (Class|IreneCharacter|HPFullRecovery)))

(event Input|KeyboardEvents|Ctrl6
  (params (Key :type Key%20Structure :default "None"))
  (:Pressed
    (Class|IreneCharacter|SetIsPlay)
    (Class|FMODBlueprintStatics|BusStopAllEvents "/Game/FMOD/Buses/Master.Master" "ALLOWFADEOUT")
    (bind _asstgame_instance (Utilities|Casting|CastToSTGameInstance (Game|GetGameInstance)))
    (Class|STGameInstance|SetFourthSpawnPosition _asstgame_instance)
    (Class|STGameInstance|InitData _asstgame_instance)
    (Game|OpenLevel(byName) "MainFairyLab")))

(event Input|KeyboardEvents|Ctrl2
  (params (Key :type Key%20Structure :default "None"))
  (:Pressed
    (Class|FMODBlueprintStatics|BusStopAllEvents "/Game/FMOD/Buses/Master.Master" "ALLOWFADEOUT")
    (bind _asstgame_instance (Utilities|Casting|CastToSTGameInstance (Game|GetGameInstance)))
    (Class|STGameInstance|SetFirstSpawnPosition _asstgame_instance)
    (Class|STGameInstance|InitData _asstgame_instance)
    (Game|OpenLevel(byName) "MainFairyLab")))

(event Input|KeyboardEvents|Ctrl1
  (params (Key :type Key%20Structure :default "None"))
  (:Pressed
    (Class|FMODBlueprintStatics|BusStopAllEvents "/Game/FMOD/Buses/Master.Master" "ALLOWFADEOUT")
    (bind _asstgame_instance (Utilities|Casting|CastToSTGameInstance (Game|GetGameInstance)))
    (Class|STGameInstance|InitData _asstgame_instance)
    (Game|OpenLevel(byName) "MainTitle")))

(event Input|KeyboardEvents|Ctrl4
  (params (Key :type Key%20Structure :default "None"))
  (:Pressed
    (Class|IreneCharacter|SetIsPlay)
    (Class|FMODBlueprintStatics|BusStopAllEvents "/Game/FMOD/Buses/Master.Master" "ALLOWFADEOUT")
    (bind _asstgame_instance (Utilities|Casting|CastToSTGameInstance (Game|GetGameInstance)))
    (Class|STGameInstance|SetSecondSpawnPosition _asstgame_instance)
    (Class|STGameInstance|InitData _asstgame_instance)
    (Game|OpenLevel(byName) "MainFairyLab")))

(event Input|KeyboardEvents|Ctrl5
  (params (Key :type Key%20Structure :default "None"))
  (:Pressed
    (Class|IreneCharacter|SetIsPlay)
    (Class|FMODBlueprintStatics|BusStopAllEvents "/Game/FMOD/Buses/Master.Master" "ALLOWFADEOUT")
    (bind _asstgame_instance (Utilities|Casting|CastToSTGameInstance (Game|GetGameInstance)))
    (Class|STGameInstance|SetThirdSpawnPosition _asstgame_instance)
    (Class|STGameInstance|InitData _asstgame_instance)
    (Game|OpenLevel(byName) "MainFairyLab")))

(fn ConstructionScript)

(fn StartHitStop
  (params (Duration :type Float%20%28single-precision%29))
  (Variables|Default|SetIsTimeStopping true)
  (Variables|Default|SetCustomTimeDilation 0.0)
  (Utilities|Time|SetTimerbyFunctionName 0 "EndHitStop" Duration))

(fn RadialBlurStart
  (params (Duration :type Float%20%28single-precision%29))
  (Rendering|Material|SetScalarParameterValue "/Game/UI/RadialBlur/RadialBlurCollection.RadialBlurCollection" "Blur" 0.0 :!class /Script/Engine.KismetMaterialLibrary)
  (Utilities|Time|SetTimerbyFunctionName 0 "RadialBlurEnd" Duration))

(fn RadialBlurEnd
  (Rendering|Material|SetScalarParameterValue "/Game/UI/RadialBlur/RadialBlurCollection.RadialBlurCollection" "Blur" 0.0 :!class /Script/Engine.KismetMaterialLibrary))

(fn EndHitStop
  (Variables|Default|SetCustomTimeDilation 1.0)
  (Variables|Default|SetCameraShakeOn true))