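; BP_Ghost1 is an afterimage actor meant to leave a fading, frozen-pose copy of a skeletal mesh.
; Its unwired logic copies a pose onto a PoseableMesh and creates dynamic instances for three material slots.
; An Opacity timeline, also unwired, would fade material arrays, only one of which that setup fills, then destroy the actor.
; Init_Event and the construction script are empty, so none of this runs.
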(event Custom|Init_Event
  (params (Gost_M :type Skeletal%20Mesh%20Component%20Object%20Reference%20%28by%20ref%29)))

(fn ConstructionScript)