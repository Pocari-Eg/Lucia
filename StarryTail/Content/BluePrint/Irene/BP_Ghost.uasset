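; BP_Ghost is an afterimage actor that freezes a copy of a skeletal mesh's pose on a poseable mesh.
; Init_Event copies the pose from the supplied mesh, swaps the first three material slots to dynamic instances, stores them in arrays, and starts the Opacity timeline.
; The timeline's update writes the Opacity parameter to those instances, and its finish destroys the actor.
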(event Custom|Init_Event
  (params (Mash :type Skeletal%20Mesh%20Component%20Object%20Reference))
  (bind _poseablemesh (Variables|Default|GetPoseableMesh))
  (bind _poseablemesh_2 (Variables|Default|GetPoseableMesh))
  (bind _returnvalue (Rendering|Material|GetMaterial _poseablemesh_2 2))
  (Class|PoseableMeshComponent|CopyPosefromSkeletalComponent (Variables|Default|GetPoseableMesh) Mash)
  (for _array_element (Utilities|Array|MakeArray _returnvalue)
    (Utilities|FlowControl|Sequence
      (:then_0
        (bind _returnvalue_2 (Rendering|Material|CreateDynamicMaterialInstance (Rendering|Material|GetMaterial (Variables|Default|GetPoseableMesh) 0) "None" "None" :!class /Script/Engine.KismetMaterialLibrary))
        (bind _output_get (Variables|Default|SetGhost_Tail_M_3 _returnvalue_2))
        (Utilities|FlowControl|Sequence
          (:then_0
            (Utilities|Array|Add (Variables|Default|GetNewVar_3) _output_get))
          (:then_1
            (Rendering|Material|SetMaterial _poseablemesh 0 _returnvalue_2))))
      (:then_1
        (bind _returnvalue_3 (Rendering|Material|CreateDynamicMaterialInstance (Rendering|Material|GetMaterial (Variables|Default|GetPoseableMesh) 1) "None" "None" :!class /Script/Engine.KismetMaterialLibrary))
        (bind _output_get_2 (Variables|Default|SetGhost_Tail_M_2 _returnvalue_3))
        (Utilities|FlowControl|Sequence
          (:then_0
            (Utilities|Array|Add (Variables|Default|GetNewVar_2) _output_get_2))
          (:then_1
            (Rendering|Material|SetMaterial _poseablemesh 1 _returnvalue_3))))
      (:then_2
        (bind _returnvalue_4 (Rendering|Material|CreateDynamicMaterialInstance _returnvalue "None" "None" :!class /Script/Engine.KismetMaterialLibrary))
        (bind _output_get_3 (Variables|Default|SetGhost_Tail_M_1 _returnvalue_4))
        (Utilities|FlowControl|Sequence
          (:then_0
            (Utilities|Array|Add (Variables|Default|GetNewVar_1) _output_get_3))
          (:then_1
            (Rendering|Material|SetMaterial _poseablemesh 2 _returnvalue_4))))))
  (Components|Timeline|PlayfromStart (Variables|Colors|GetOpacity)))

(fn ConstructionScript)