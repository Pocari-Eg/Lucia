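; Bellyfish flying monster Blueprint that handles material effects, fly-distance tracking and the stack widget.
; Dynamic stone and body materials receive timeline-driven parameters on shield destruction and, after a short delay, on death.
; Each tick, a line trace from the capsule measures the vertical gap to the hit, setting fly distance to the maximum minus that gap.
; Stack events update the target widget's count and trigger its animation or explosion.
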(event EventBeginPlay
  (bind _mesh (Variables|Character|GetMesh))
  (bind _returnvalue (Rendering|Material|CreateDynamicMaterialInstance _mesh 0 "/Game/Animation/Monster/Bellyfish/Mesh/Texture/MI_Bellyfish_Stone.MI_Bellyfish_Stone" "None" :!class /Script/Engine.PrimitiveComponent))
  (bind _returnvalue_2 (Rendering|Material|CreateDynamicMaterialInstance _mesh 1 "/Game/Animation/Monster/Bellyfish/Mesh/Texture/MI_Bellyfish_Body.MI_Bellyfish_Body" "None" :!class /Script/Engine.PrimitiveComponent)))

(event EventTick
  (params (DeltaSeconds :type Float%20%28single-precision%29))
  (bind _capsulecomponent (Variables|Default|GetCapsuleComponent))
  (bind _returnvalue (Transformation|GetWorldLocation _capsulecomponent))
  (bind _outhit (Collision|LineTraceByChannel _returnvalue (+ _returnvalue (* (Math|Vector|RotateVector (Math|Vector|GetUpVector _capsulecomponent) "180.000000, 0, 0") 1e+03)) "TraceTypeQuery1" false 0 "None" true "(R=1.000000,G=0.000000,B=0.000000,A=1.000000)" "(R=0.000000,G=1.000000,B=0.000000,A=1.000000)" 0.0))
  (bind _returnvalue_2 (Class|Bellyfish|GetMaxFlyDistance))
  (Class|Bellyfish|SetFlyDistance (- _returnvalue_2 (- (.z (Transformation|GetWorldLocation (Variables|Default|GetCapsuleComponent))) (.z (.Location (Collision|BreakHitResult _outhit)))))))

(event EventShieldDestroyEvent
  (bind _새_트랙_0 (Timeline|타임라인_0 Play)
    (:Update
      (Rendering|Material|SetScalarParameterValue (stale EventBeginPlay _returnvalue) "LV2_Power" _새_트랙_0 :!class /Script/Engine.MaterialInstanceDynamic))))

(event EventMonsterDeadEvent
  (Utilities|FlowControl|Delay 1.0)
  (bind _spawn (Timeline|타임라인_1 PlayFromStart)
    (:Update
      (Rendering|Material|SetScalarParameterValue (stale EventBeginPlay _returnvalue) "Dead_" _spawn :!class /Script/Engine.MaterialInstanceDynamic))))

(event EventExplodeStackEvent
  (bind _asbp_target_wdiget (Utilities|Casting|CastToBP_TargetWdiget (UserInterface|GetUserWidgetObject (Variables|Default|GetStackWidget))))
  (Default|CallStackExplode _asbp_target_wdiget self))

(event EventOnStackCountEvent
  (bind _asbp_target_wdiget (Utilities|Casting|CastToBP_TargetWdiget (UserInterface|GetUserWidgetObject (Variables|Default|GetStackWidget))))
  (bind _returnvalue (Class|Monster|GetCurStackCount))
  (Variables|/Game/UI/BluePrint/Monster/BP_TargetWdiget.BP_TargetWdiget_C|SetStackCount _asbp_target_wdiget _returnvalue)
  (Default|CallStackAnmationDispatcher _asbp_target_wdiget))

(fn ConstructionScript)