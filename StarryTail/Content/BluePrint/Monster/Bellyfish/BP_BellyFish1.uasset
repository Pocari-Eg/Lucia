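; Bellyfish flying monster Blueprint that maintains its fly distance and shows stack feedback through a widget.
; Each tick, it line-traces along the capsule's rotated up vector and sets fly distance to the maximum minus the vertical gap to the hit.
; Stack count and explode events forward to BP_TargetWdiget in StackWidget, triggering its animation or explosion.
; BeginPlay creates dynamic material instances for two mesh slots.
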(event EventBeginPlay
  (bind _mesh (Variables|Character|GetMesh))
  (Rendering|Material|CreateDynamicMaterialInstance _mesh 0 "/Game/Animation/Monster/Bellyfish/Mesh/Texture/MI_Bellyfish_Stone_E_2.MI_Bellyfish_Stone_E_2" "None" :!class /Script/Engine.PrimitiveComponent)
  (Rendering|Material|CreateDynamicMaterialInstance _mesh 1 "/Game/Animation/Monster/Bellyfish/Mesh/Texture/NewMaterial_2_Inst1.NewMaterial_2_Inst1" "None" :!class /Script/Engine.PrimitiveComponent))

(event EventTick
  (params (DeltaSeconds :type Float%20%28single-precision%29))
  (bind _capsulecomponent (Variables|Default|GetCapsuleComponent))
  (bind _returnvalue (Transformation|GetWorldLocation _capsulecomponent))
  (bind _outhit (Collision|LineTraceByChannel _returnvalue (+ _returnvalue (* (Math|Vector|RotateVector (Math|Vector|GetUpVector _capsulecomponent) "180.000000, 0, 0") 1e+03)) "TraceTypeQuery1" false 0 "None" true "(R=1.000000,G=0.000000,B=0.000000,A=1.000000)" "(R=0.000000,G=1.000000,B=0.000000,A=1.000000)" 0.0))
  (bind _returnvalue_2 (Class|Bellyfish|GetMaxFlyDistance))
  (Class|Bellyfish|SetFlyDistance (- _returnvalue_2 (- (.z (Transformation|GetWorldLocation (Variables|Default|GetCapsuleComponent))) (.z (.Location (Collision|BreakHitResult _outhit)))))))

(event EventOnStackCountEvent
  (bind _asbp_target_wdiget (Utilities|Casting|CastToBP_TargetWdiget (UserInterface|GetUserWidgetObject (Variables|Default|GetStackWidget))))
  (bind _returnvalue (Class|Monster|GetCurStackCount))
  (Variables|/Game/UI/BluePrint/Monster/BP_TargetWdiget.BP_TargetWdiget_C|SetStackCount _asbp_target_wdiget _returnvalue)
  (Default|CallStackAnmationDispatcher _asbp_target_wdiget))

(event EventExplodeStackEvent
  (bind _asbp_target_wdiget (Utilities|Casting|CastToBP_TargetWdiget (UserInterface|GetUserWidgetObject (Variables|Default|GetStackWidget))))
  (Default|CallStackExplode _asbp_target_wdiget self))

(fn ConstructionScript)