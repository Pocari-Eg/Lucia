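; Morbit monster Blueprint that handles attribute-based appearance, spawn, hit and death visuals, and hit stop.
; The construction script picks the mesh material by monster attribute, with Fire also swapping the skeletal mesh.
; Spawning creates two dynamic instances of the None-attribute material, whose dissolve and hit parameters are animated by timelines; death ends by destroying the actor.
; StartHitStop freezes the actor through custom time dilation until a timer calls EndHitStop.
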(event EventMonsterDeadEvent
  ;[1 1 1] Material_Instance
  (bind _dead (Timeline|타임라인_1 PlayFromStart)
    (:Update
      (Rendering|Material|SetScalarParameterValue (stale EventOnSpawnEffectEvent _returnvalue) "Dead_" _dead :!class /Script/Engine.MaterialInstanceDynamic)
      (Input|EnableInput 0))
    (:Finished
      (Actor|DestroyActor))))

(event EventHitStopEvent
  ;[1 1 1] Material_Instance
  (bind _hit (Timeline|타임라인_0 PlayFromStart)
    (:Update
      (Rendering|Material|SetScalarParameterValue (stale EventOnSpawnEffectEvent _returnvalue) "Hit_Power" _hit :!class /Script/Engine.MaterialInstanceDynamic)
      (Input|EnableInput 0))))

(event EventOnSpawnEffectEvent
  (bind _mesh (Variables|Character|GetMesh))
  ;[1 1 1] Material_Instance
  (bind _returnvalue (Rendering|Material|CreateDynamicMaterialInstance _mesh 0 "/Game/Model/Monster/Morbit/Material/MI_Morbit_Non_.MI_Morbit_Non_" "None" :!class /Script/Engine.PrimitiveComponent))
  (bind _returnvalue_2 (Rendering|Material|CreateDynamicMaterialInstance _mesh 1 "/Game/Model/Monster/Morbit/Material/MI_Morbit_Non_.MI_Morbit_Non_" "None" :!class /Script/Engine.PrimitiveComponent))
  (bind _spawn (Timeline|타임라인_2 Play)
    (:Update
      (Rendering|Material|SetScalarParameterValue _returnvalue_2 "Dead_" _spawn :!class /Script/Engine.MaterialInstanceDynamic))))

(fn ConstructionScript
  (bind _mesh (Variables|Character|GetMesh))
  (switch Utilities|FlowControl|Switch|SwitchonEAttributeKeyword (.monsterattribute (Variables|Default|GetMonsterInfo))
    (:e_None
      (Rendering|Material|SetMaterial _mesh 0 "/Game/Model/Monster/Morbit/Material/MI_Morbit_Non_.MI_Morbit_Non_"))
    (:e_Fire
      (Class|SkinnedMeshComponent|SetSkeletalMesh _mesh "/Game/Model/Monster/Morbit/Mash/M_FireM_rig__1_.M_FireM_rig__1_" true)
      (Rendering|Material|SetMaterial _mesh 0 "/Game/Model/Monster/Morbit/Material/MI_Morbit_Fire.MI_Morbit_Fire"))
    (:e_Water
      (Rendering|Material|SetMaterial _mesh 0 "/Game/Model/Monster/Morbit/Material/MI_Morbit_Water.MI_Morbit_Water"))
    (:e_Thunder
      (Rendering|Material|SetMaterial _mesh 0 0))))

(fn StartHitStop
  (params (Duration :type Float%20%28single-precision%29))
  (Variables|Default|SetCustomTimeDilation 0.0)
  (Utilities|Time|SetTimerbyFunctionName 0 "EndHitStop" Duration))

(fn EndHitStop
  (Variables|Default|SetCustomTimeDilation 1.0))