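; BP_MorbitCode8 is a Morbit monster Blueprint, under BP_Thunder, that drives electric material effects for spawn, hit and death.
; The spawn event creates dynamic instances of MI_Morbit_Electric1 on two mesh slots, which the other events reuse.
; Timelines animate Dead_ for spawn and death and Hit_Power for hit stop, calling EnableInput on every update.
; StartHitStop is empty, and the construction script only calls its parent.
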(event EventMonsterDeadEvent
  ;[1 1 1] Material_Instance
  (bind _dead (Timeline|타임라인_4 PlayFromStart)
    (:Update
      (Rendering|Material|SetScalarParameterValue (stale EventOnSpawnEffectEvent _returnvalue) "Dead_" _dead :!class /Script/Engine.MaterialInstanceDynamic)
      (Input|EnableInput 0))))

(event EventHitStopEvent
  ;[1 1 1] Material_Instance
  (bind _hit (Timeline|타임라인_3 PlayFromStart)
    (:Update
      (Rendering|Material|SetScalarParameterValue (stale EventOnSpawnEffectEvent _returnvalue) "Hit_Power" _hit :!class /Script/Engine.MaterialInstanceDynamic)
      (Input|EnableInput 0))))

(event EventOnSpawnEffectEvent
  (bind _mesh (Variables|Character|GetMesh))
  ;[1 1 1] Material_Instance
  (bind _returnvalue (Rendering|Material|CreateDynamicMaterialInstance _mesh 0 "/Game/Model/Monster/Morbit/Material/MI_Morbit_Electric1.MI_Morbit_Electric1" "None" :!class /Script/Engine.PrimitiveComponent))
  (bind _returnvalue_2 (Rendering|Material|CreateDynamicMaterialInstance _mesh 1 "/Game/Model/Monster/Morbit/Material/MI_Morbit_Electric1.MI_Morbit_Electric1" "None" :!class /Script/Engine.PrimitiveComponent))
  (bind _spawn (Timeline|타임라인_5 PlayFromStart)
    (:Update
      (Rendering|Material|SetScalarParameterValue _returnvalue_2 "Dead_" _spawn :!class /Script/Engine.MaterialInstanceDynamic)
      (Input|EnableInput 0))))

(fn ConstructionScript
  (|CallParentFunction))

(fn StartHitStop
  (params (Duration :type Float%20%28single-precision%29)))