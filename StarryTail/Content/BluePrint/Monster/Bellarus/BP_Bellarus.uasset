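; Bellarus monster Blueprint that handles visual feedback for its second phase, teleport, death and stack mechanic.
; Dynamic material instances on the mesh take phase-two power changes, alongside three activated particle systems, and a timeline-driven death effect.
; Teleport fades animate a shared Material Parameter Collection scalar, calling TelePortStart once the fade-out finishes.
; Stack events forward the count and explosion to the BP_TargetWdiget widget component for animation.
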(event EventTelePortEndEvent
  ;[1 1 1] 스킬 투명화
  (Rendering|Material|SetScalarParameterValue "/Game/BluePrint/Monster/Bellarus/MCP_Opt.MCP_Opt" "Ops" 0.0 :!class /Script/Engine.KismetMaterialLibrary)
  (bind _spawn (Timeline|타임라인_2 PlayFromStart)
    (:Update
      (Rendering|Material|SetScalarParameterValue "/Game/BluePrint/Monster/Bellarus/MCP_Opt.MCP_Opt" "Ops" _spawn :!class /Script/Engine.KismetMaterialLibrary))))

(event EventTelePortStartEvent
  ;[1 1 1] 스킬 투명화
  (Rendering|Material|SetScalarParameterValue "/Game/BluePrint/Monster/Bellarus/MCP_Opt.MCP_Opt" "Ops" 1.0 :!class /Script/Engine.KismetMaterialLibrary)
  (bind _spawn (Timeline|타임라인_1 PlayFromStart)
    (:Update
      (Rendering|Material|SetScalarParameterValue "/Game/BluePrint/Monster/Bellarus/MCP_Opt.MCP_Opt" "Ops" _spawn :!class /Script/Engine.KismetMaterialLibrary))
    (:Finished
      (Class|Bellarus|TelePortStart))))

(event EventOnSecondPhaseEvent
  ;[1 1 1] 2페이즈 시작 이벤트
  (Development|PrintText "Paese2")
  (Components|Activation|SetActive (Variables|Default|GetParticleSystem) true false)
  (Development|PrintText "spawn_particle")
  (Rendering|Material|SetScalarParameterValue (stale EventBeginPlay _returnvalue) "LV2_Power" 3.0 :!class /Script/Engine.MaterialInstanceDynamic))

(event EventExplodeStackEvent
  (bind _asbp_target_wdiget (Utilities|Casting|CastToBP_TargetWdiget (UserInterface|GetUserWidgetObject (Variables|Default|GetStackWidget))))
  (Default|CallStackExplode _asbp_target_wdiget self))

(event EventMonsterDeadEvent
  ;[1 1 1] 코멘트
  (Utilities|FlowControl|Delay 1.0)
  (bind _spawn (Timeline|타임라인_0 PlayFromStart)
    (:Update
      (Rendering|Material|SetScalarParameterValue (stale EventBeginPlay _returnvalue) "Dead_" _spawn :!class /Script/Engine.MaterialInstanceDynamic))))

(event EventBeginPlay
  (bind _mesh (Variables|Character|GetMesh))
  (Utilities|FlowControl|Sequence
    (:then_0
      (Components|Activation|Deactivate (Variables|Default|GetParticleSystem2)))
    (:then_1
      ;[1 1 1] 코멘트
      (bind _returnvalue (Rendering|Material|CreateDynamicMaterialInstance _mesh 0 "/Game/Animation/Monster/Bellarus/MI_Bellarus_Accessory.MI_Bellarus_Accessory" "None" :!class /Script/Engine.PrimitiveComponent))
      (bind _returnvalue_2 (Rendering|Material|CreateDynamicMaterialInstance _mesh 1 "/Game/Animation/Monster/Bellarus/MI_Bellarus_Body.MI_Bellarus_Body" "None" :!class /Script/Engine.PrimitiveComponent))
      (bind _returnvalue_3 (Rendering|Material|CreateDynamicMaterialInstance _mesh 2 "/Game/Animation/Monster/Bellarus/MI_Bellarus_Wing.MI_Bellarus_Wing" "None" :!class /Script/Engine.PrimitiveComponent))
      (bind _returnvalue_4 (Rendering|Material|CreateDynamicMaterialInstance _mesh 3 "/Game/Animation/Monster/Bellarus/MI_Bellarus_Accessory.MI_Bellarus_Accessory" "None" :!class /Script/Engine.PrimitiveComponent))
      (Rendering|Material|SetScalarParameterValue "/Game/BluePrint/Monster/Bellarus/MCP_Opt.MCP_Opt" "Ops" 1.0 :!class /Script/Engine.KismetMaterialLibrary)
      (Rendering|Material|SetScalarParameterValue _returnvalue_4 "LV2_Power" 2e+02 :!class /Script/Engine.MaterialInstanceDynamic))))

(event EventOnStackCountEvent
  (bind _asbp_target_wdiget (Utilities|Casting|CastToBP_TargetWdiget (UserInterface|GetUserWidgetObject (Variables|Default|GetStackWidget))))
  (bind _returnvalue (Class|Monster|GetCurStackCount))
  (Variables|/Game/UI/BluePrint/Monster/BP_TargetWdiget.BP_TargetWdiget_C|SetStackCount _asbp_target_wdiget _returnvalue)
  (Default|CallStackAnmationDispatcher _asbp_target_wdiget))

(fn ConstructionScript)