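; BP_Scientia is the Blueprint for the Scientia monster, driving its visual state through spawn, magic stone breakage and death.
; Spawn and death events create dynamic materials for hair, body and wing, then animate their "Dead_" parameter with timelines.
; Three crush events swap the body to progressively broken materials as each magic stone stage shatters.
; BeginPlay sets the max barrier, and Tick writes a fixed-index palette color to a material parameter collection.
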(event EventBeginPlay
  (Class|Scientia|SetMaxBarrierValue))

(event Collision|EventActorBeginOverlap
  (params (OtherActor :type Actor%20Object%20Reference)))

(event EventMonsterDeadEvent
  (bind _mesh (Variables|Character|GetMesh))
  (bind _returnvalue (Rendering|Material|CreateDynamicMaterialInstance _mesh 0 "/Game/Model/Monster/Scientia/Material/MI_Scientia_Hair.MI_Scientia_Hair" "None" :!class /Script/Engine.PrimitiveComponent))
  (bind _returnvalue_2 (Rendering|Material|CreateDynamicMaterialInstance _mesh 1 "/Game/Model/Monster/Scientia/Material/MI_Scientia_Body_Break3.MI_Scientia_Body_Break3" "None" :!class /Script/Engine.PrimitiveComponent))
  (bind _returnvalue_3 (Rendering|Material|CreateDynamicMaterialInstance _mesh 2 "/Game/Model/Monster/Scientia/Material/MI_Scientia_Wing.MI_Scientia_Wing" "None" :!class /Script/Engine.PrimitiveComponent))
  (bind _dead (Timeline|타임라인_1 PlayFromStart)
    (:Update
      (Rendering|Material|SetScalarParameterValue _returnvalue_3 "Dead_" _dead :!class /Script/Engine.MaterialInstanceDynamic))))

(event EventOnSpawnEffectEvent
  (bind _mesh (Variables|Character|GetMesh))
  (bind _returnvalue (Rendering|Material|CreateDynamicMaterialInstance _mesh 0 "/Game/Model/Monster/Scientia/Material/MI_Scientia_Hair.MI_Scientia_Hair" "None" :!class /Script/Engine.PrimitiveComponent))
  (bind _returnvalue_2 (Rendering|Material|CreateDynamicMaterialInstance _mesh 1 "/Game/Model/Monster/Scientia/Material/MI_Scientia_Body.MI_Scientia_Body" "None" :!class /Script/Engine.PrimitiveComponent))
  (bind _returnvalue_3 (Rendering|Material|CreateDynamicMaterialInstance _mesh 2 "/Game/Model/Monster/Scientia/Material/MI_Scientia_Wing.MI_Scientia_Wing" "None" :!class /Script/Engine.PrimitiveComponent))
  (bind _spawn (Timeline|타임라인_0 PlayFromStart)
    (:Update
      (Rendering|Material|SetScalarParameterValue _returnvalue_3 "Dead_" _spawn :!class /Script/Engine.MaterialInstanceDynamic))))

(event EventFirstCrushedEvent
  ;[1 1 1] 1단계 마법석 부숴짐
  (Rendering|Material|CreateDynamicMaterialInstance (Variables|Character|GetMesh) 1 "/Game/Model/Monster/Scientia/Material/MI_Scientia_Body_Break1.MI_Scientia_Body_Break1" "None" :!class /Script/Engine.PrimitiveComponent))

(event EventSecondCrushedEvent
  ;[1 1 1] 2단계 마법석 부숴짐
  (Rendering|Material|CreateDynamicMaterialInstance (Variables|Character|GetMesh) 1 "/Game/Model/Monster/Scientia/Material/MI_Scientia_Body_Break2.MI_Scientia_Body_Break2" "None" :!class /Script/Engine.PrimitiveComponent))

(event EventThirdCrushedEvent
  ;[1 1 1] 3단계 마법석 부숴짐
  (Rendering|Material|CreateDynamicMaterialInstance (Variables|Character|GetMesh) 1 "/Game/Model/Monster/Scientia/Material/MI_Scientia_Body_Break3.MI_Scientia_Body_Break3" "None" :!class /Script/Engine.PrimitiveComponent))

(event EventTick
  (params (DeltaSeconds :type Float%20%28single-precision%29))
  (Utilities|FlowControl|Sequence
    (:then_0
      (bind _output_get (Variables|Default|SetColor_S (Utilities|Array|Get(acopy) (Utilities|Array|MakeArray "(R=1.000000,G=1.000000,B=1.000000,A=1.000000)" "(R=1.000000,G=0.000000,B=0.000000,A=1.000000)" "(R=0.000000,G=0.684300,B=1.000000,A=1.000000)" "(R=1.000000,G=0.000000,B=0.836574,A=1.000000)") (Math|Conversions|ToInteger(Byte) 0)))))
    (:then_1
      (Rendering|Material|SetVectorParameterValue "/Game/Model/Monster/Scientia/Material/MPC_Scientia_Color.MPC_Scientia_Color" "Color" _output_get :!class /Script/Engine.KismetMaterialLibrary))))

(fn ConstructionScript)