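; BP_PartsObject is a parts object actor whose Mesh bobs up and down in the level.
; On BeginPlay it stores the mesh's relative location and plays the Hover timeline.
; Each update offsets Z from that location by lerping toward ZMovementDistance with the timeline alpha, with ZMovementSpeed as the play rate.
; Overlap and Tick events are empty.
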(event EventBeginPlay
  ;[1 1 1] Mesh 위아래 움직임
  (Variables|Default|SetNewMeshLocation (Variables|/Script/Engine.SceneComponent|GetRelativeLocation (Variables|Character|GetMesh)))
  (bind _alpha (Timeline|Hover Play)
    (:Update
      (Components|Timeline|SetPlayRate (Variables|Default|GetHover) (Variables|Default|GetZMovementSpeed))
      (Transformation|SetRelativeLocation (Variables|Character|GetMesh) (Math|Vector|MakeVector (.X (Math|Vector|BreakVector (Variables|Default|GetNewMeshLocation))) (.Y (Math|Vector|BreakVector (Variables|Default|GetNewMeshLocation))) (+ (.Z (Math|Vector|BreakVector (Variables|Default|GetNewMeshLocation))) (Math|Float|Lerp 0.0 (Variables|Default|GetZMovementDistance) _alpha))) false false))))

(event Collision|EventActorBeginOverlap
  (params (OtherActor :type Actor%20Object%20Reference)))

(event EventTick
  (params (DeltaSeconds :type Float%20%28single-precision%29)))

(fn ConstructionScript)