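; Trigger box that shows a tutorial when BP_IreneCharacter overlaps it, with the step selected by PLAY.
; CheckTuto reads and sets per-step flags in STGameInstance, so each fires once.
; SPACE swaps the TutorialWidget Move prompt for Space on entry and stops Move again on exit.
; The monster and room steps show tutorial info, destroy the trigger and freeze time with zero global time dilation.
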(event OnComponentBeginOverlap(Box)
  (params (OverlappedComponent :type Primitive%20Component%20Object%20Reference) (OtherActor :type Actor%20Object%20Reference) (OtherComp :type Primitive%20Component%20Object%20Reference) (OtherBodyIndex :type Integer) (bFromSweep :type Boolean) (SweepResult :type Hit%20Result%20Structure%20%28by%20ref%29))
  (Utilities|Casting|CastToBP_IreneCharacter OtherActor)
  (switch Utilities|FlowControl|Switch|SwitchonEPlayTuto (Variables|Default|GetPLAY)
    (:SPACE
      (bind _isplay (CallFunction|CheckTuto))
      (if (not _isplay)
        (bind _foundwidgets (Widget|GetAllWidgetsOfClass "/Script/StarryTail.TutorialWidget" true))
        (for _array_element _foundwidgets
          (Class|TutorialWidget|TrystopPlay _array_element "Move")
          (Class|TutorialWidget|TryPlay _array_element "Space"))))
    (:beforAcrossmonster
      (bind _isplay_2 (CallFunction|CheckTuto 1))
      (if (not _isplay_2)
        (bind _foundwidgets_2 (Widget|GetAllWidgetsOfClass "/Script/StarryTail.TutorialWidget" true))
        (for _array_element_2 _foundwidgets_2
          (Class|TutorialWidget|TryTutoInfo _array_element_2 "beforAcrossmonster")
          (Actor|DestroyActor)
          (Utilities|Time|SetGlobalTimeDilation 0.0))))
    (:acrossmonster
      (bind _isplay_3 (CallFunction|CheckTuto 2))
      (if (not _isplay_3)
        (bind _foundwidgets_3 (Widget|GetAllWidgetsOfClass "/Script/StarryTail.TutorialWidget" true))
        (for _array_element_3 _foundwidgets_3
          (Class|TutorialWidget|TryTutoInfo _array_element_3 "acrossmonster")
          (Actor|DestroyActor)
          (Utilities|Time|SetGlobalTimeDilation 0.0))))
    (:stepinroom
      (bind _isplay_4 (CallFunction|CheckTuto 3))
      (if (not _isplay_4)
        (bind _foundwidgets_4 (Widget|GetAllWidgetsOfClass "/Script/StarryTail.TutorialWidget" true))
        (for _array_element_4 _foundwidgets_4
          (Class|TutorialWidget|TryTutoInfo _array_element_4 "stepinroom")
          (Actor|DestroyActor)
          (Utilities|Time|SetGlobalTimeDilation 0.0))))))

(event OnComponentEndOverlap(Box)
  (params (OverlappedComponent :type Primitive%20Component%20Object%20Reference) (OtherActor :type Actor%20Object%20Reference) (OtherComp :type Primitive%20Component%20Object%20Reference) (OtherBodyIndex :type Integer))
  (Utilities|Casting|CastToBP_IreneCharacter OtherActor)
  (switch Utilities|FlowControl|Switch|SwitchonEPlayTuto (Variables|Default|GetPLAY)
    (:SPACE
      (bind _isplay (CallFunction|CheckTuto 4))
      (if (not _isplay)
        (bind _foundwidgets (Widget|GetAllWidgetsOfClass "/Script/StarryTail.TutorialWidget" true))
        (for _array_element _foundwidgets
          (Class|TutorialWidget|TrystopPlay _array_element "Move"))))))

(fn ConstructionScript)

(fn CheckTuto
  (params (num :type Integer))
  (bind _asstgame_instance (Utilities|Casting|CastToSTGameInstance (Game|GetGameInstance)))
  (bind _returnvalue (Class|STGameInstance|GetTutorialState _asstgame_instance num))
  (if _returnvalue
    (return true)
    (else
      (Class|STGameInstance|SetTutorial _asstgame_instance num true)
      (return false))))