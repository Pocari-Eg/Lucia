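; Level trigger volume that moves the game to the map named in NextLevel.
; Any Box overlap binds the next-level dispatcher, pauses the game, fades out Master-bus audio, switches to UI-only input and plays the player Irene's fade-in animation.
; An overlapping IreneCharacter also has all its timers cleared.
; When the dispatcher fires, NextLevelEvent resets STGameInstance data through InitData and opens the level.
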(event OnComponentBeginOverlap(Box)
  (params (OverlappedComponent :type Primitive%20Component%20Object%20Reference) (OtherActor :type Actor%20Object%20Reference) (OtherComp :type Primitive%20Component%20Object%20Reference) (OtherBodyIndex :type Integer) (bFromSweep :type Boolean) (SweepResult :type Hit%20Result%20Structure%20%28by%20ref%29))
  ;[1 1 1] Fade In Out
  (Utilities|FlowControl|Sequence
    (:then_0
      (EventDispatchers|BindEventtoNextLevelEventDispatcher (delegate Custom|NextLevelEvent))
      (Game|SetGamePaused true)
      (Class|FMODBlueprintStatics|BusStopAllEvents "/Game/FMOD/Buses/Master.Master" "ALLOWFADEOUT")
      (Input|SetInputModeUIOnly (Game|GetPlayerController 0) 0 "DoNotLock")
      (bind _asirene_character (Utilities|Casting|CastToIreneCharacter (Game|GetPlayerCharacter 0)))
      (Class|IreneCharacter|PlayFadeinAnimation _asirene_character))
    (:then_1
      (bind _asirene_character_2 (Utilities|Casting|CastToIreneCharacter OtherActor))
      (Class|IreneCharacter|AllTimerClear _asirene_character_2))))

(event Custom|NextLevelEvent
  ;[1 1 1] Fade In Out
  (bind _asstgame_instance (Utilities|Casting|CastToSTGameInstance (Game|GetGameInstance)))
  (Class|STGameInstance|InitData _asstgame_instance)
  (Game|OpenLevel(byName) (Variables|Default|GetNextLevel)))

(fn ConstructionScript)