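; BP_AttributeObject is a puzzle object that visually reflects its elemental attribute: none, fire, water or thunder.
; BeginPlay creates dynamic instances of MI_PuzzleToolBase on the Plate, Crystal and object meshes.
; MaterialChange sets their emissive color per element and animates intensity through one timeline, with a second timeline playing for NONE.
; It also deactivates the previous particle effect and attaches the attribute's emitter above the object mesh.
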(event Collision|EventActorBeginOverlap
  (params (OtherActor :type Actor%20Object%20Reference)))

(event EventTick
  (params (DeltaSeconds :type Float%20%28single-precision%29)))

(event EventBeginPlay
  (bind _asstatic_mesh_component (Utilities|Casting|CastToStaticMeshComponent (Variables|/Script/Engine.Actor|GetRootComponent (Variables|Default|GetPlate))))
  (Variables|Default|SetPlateMesh _asstatic_mesh_component)
  (bind _asskeletal_mesh_component (Utilities|Casting|CastToSkeletalMeshComponent (Variables|/Script/Engine.Actor|GetRootComponent (Variables|Default|GetCrystal))))
  (Variables|Default|SetCrystalMesh _asskeletal_mesh_component)
  ;[1 1 1] 코멘트
  (bind _returnvalue (Rendering|Material|CreateDynamicMaterialInstance (Variables|Default|GetPlateMesh) 0 "/Game/3DEnvironment/Asset/R0R1_LibraryAllMap/PuzzleRoom/PuzzleTool/MI_PuzzleToolBase.MI_PuzzleToolBase" "None" :!class /Script/Engine.PrimitiveComponent))
  (bind _returnvalue_2 (Rendering|Material|CreateDynamicMaterialInstance (Variables|Default|GetCrystalMesh) 0 "/Game/3DEnvironment/Asset/R0R1_LibraryAllMap/PuzzleRoom/PuzzleTool/MI_PuzzleToolBase.MI_PuzzleToolBase" "None" :!class /Script/Engine.PrimitiveComponent))
  (bind _returnvalue_3 (Rendering|Material|CreateDynamicMaterialInstance (Variables|Default|GetObjectMesh) 0 "/Game/3DEnvironment/Asset/R0R1_LibraryAllMap/PuzzleRoom/PuzzleTool/MI_PuzzleToolBase.MI_PuzzleToolBase" "None" :!class /Script/Engine.PrimitiveComponent)))

(event EventMaterialChange
  ;[1 1 1] 코멘트
  (Utilities|FlowControl|Sequence
    (:then_0
      (bind _returnvalue (Class|AttributeObject|GetAttribute))
      (switch Utilities|FlowControl|Switch|SwitchonEAttributeKeyword _returnvalue
        (:e_None
          (Utilities|FlowControl|Sequence
            (:then_0
              (bind _새_트랙_0 (Timeline|타임라인_0 Stop)
                (:Update
                  (Rendering|Material|SetScalarParameterValue (stale EventBeginPlay _returnvalue_3) "Emisive intersity" _새_트랙_0 :!class /Script/Engine.MaterialInstanceDynamic))))
            (:then_1
              (bind _새_트랙_0_2 (Timeline|타임라인_1 PlayFromStart)
                (:Update
                  (Rendering|Material|SetScalarParameterValue (stale EventBeginPlay _returnvalue_3) "Emisive intersity" _새_트랙_0_2 :!class /Script/Engine.MaterialInstanceDynamic))))))
        (:e_Fire
          (Rendering|Material|SetVectorParameterValue (stale EventBeginPlay _returnvalue_2) "EmissiveColor" "(R=1.000000,G=0.021601,B=0.000000,A=1.000000)" :!class /Script/Engine.MaterialInstanceDynamic)
          (Timeline|타임라인_0 PlayFromStart))
        (:e_Water
          (Rendering|Material|SetVectorParameterValue (stale EventBeginPlay _returnvalue) "EmissiveColor" "(R=0.000000,G=0.477345,B=1.000000,A=1.000000)" :!class /Script/Engine.MaterialInstanceDynamic)
          (Timeline|타임라인_0 PlayFromStart))
        (:e_Thunder
          (Rendering|Material|SetVectorParameterValue (stale EventBeginPlay _returnvalue_3) "EmissiveColor" "(R=0.710431,G=0.000000,B=1.000000,A=1.000000)" :!class /Script/Engine.MaterialInstanceDynamic)
          (Timeline|타임라인_0 PlayFromStart))))
    (:then_1
      (Utilities|IsValid (Variables|Default|GetPuz_ef)
        (:Is%20Valid
          (Components|Activation|Deactivate (Variables|Default|GetPuz_ef)))
        (:Is%20Not%20Valid
          _))
      (bind _returnvalue_2 (Effects|SpawnEmitterAttached (Utilities|Array|Get(acopy) (Utilities|Array|MakeArray 0 "/Game/Effect/VFX_Background/PS_Puzzel_Fire.PS_Puzzel_Fire" "/Game/Effect/VFX_Background/PS_Puzzel_Water.PS_Puzzel_Water" "/Game/Effect/VFX_Background/PS_Puzzel_Thunder.PS_Puzzel_Thunder") (Math|Conversions|ToInteger(Byte) _returnvalue)) (Variables|Default|GetObjectMesh) "None" "0.000000, 0,320.000000"))
      (Variables|Default|SetPuz_ef _returnvalue_2))))

(fn ConstructionScript)